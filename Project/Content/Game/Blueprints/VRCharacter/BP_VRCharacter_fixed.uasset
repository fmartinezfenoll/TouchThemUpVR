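; VR player character that maps Enhanced Input actions to movement, teleportation and two-handed grabbing.
; Move input feeds CharacterMoveForward, while teleport input begins teleport on the Teleportation component above a small threshold and ends it below that or on completion.
; Each grab axis drives its hand pose, fires a grab press near full pull, and releases and resets the pose on cancel or completion.
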(event Input|EnhancedActionEvents|EnhancedInputActionIA_VR_Move
  (params (ActionValue :type Float%20%28double-precision%29) (ElapsedSeconds :type Float%20%28double-precision%29) (TriggeredSeconds :type Float%20%28double-precision%29) (InputAction :type Input%20Action%20Object%20Reference :default "/Game/Game/Blueprints/Input/IA_VR_Move.IA_VR_Move"))
  (Class|VRCharacterBase|CharacterMoveForward ActionValue))

(event Input|EnhancedActionEvents|EnhancedInputActionIA_VR_Teleport
  (params (ActionValue :type Float%20%28double-precision%29) (ElapsedSeconds :type Float%20%28double-precision%29) (TriggeredSeconds :type Float%20%28double-precision%29) (InputAction :type Input%20Action%20Object%20Reference :default "/Game/Game/Blueprints/Input/IA_VR_Teleport.IA_VR_Teleport"))
  (bind _teleportation (Variables|Default|GetTeleportation))
  (:Triggered
    (if (>= ActionValue 0.1)
      (Class|Teleportation|BeginTeleport _teleportation 0.0)
      (else
        (Class|Teleportation|EndTeleport _teleportation :!label _label))))
  (:Completed
    (goto _label)))

(event Input|EnhancedActionEvents|EnhancedInputActionIA_VR_Grab_Left
  (params (ActionValue :type Float%20%28double-precision%29) (ElapsedSeconds :type Float%20%28double-precision%29) (TriggeredSeconds :type Float%20%28double-precision%29) (InputAction :type Input%20Action%20Object%20Reference :default "/Game/Game/Blueprints/Input/IA_VR_Grab_Left.IA_VR_Grab_Left"))
  (:Triggered
    (Class|VRCharacterBase|UpdateLeftHandPose 0.0 ActionValue)
    (if (>= ActionValue 0.8)
      (Class|VRCharacterBase|LeftGrabPressed)))
  (:Canceled
    (Class|VRCharacterBase|LeftGrabReleased :!label _label)
    (Class|VRCharacterBase|UpdateLeftHandPose 0.0 0.0))
  (:Completed
    (goto _label)))

(event Input|EnhancedActionEvents|EnhancedInputActionIA_VR_Grab_Right
  (params (ActionValue :type Float%20%28double-precision%29) (ElapsedSeconds :type Float%20%28double-precision%29) (TriggeredSeconds :type Float%20%28double-precision%29) (InputAction :type Input%20Action%20Object%20Reference :default "/Game/Game/Blueprints/Input/IA_VR_Grab_Right.IA_VR_Grab_Right"))
  (:Triggered
    (Class|VRCharacterBase|UpdateRightHandPose 0.0 ActionValue)
    (if (>= ActionValue 0.8)
      (Class|VRCharacterBase|RightGrabPressed)))
  (:Canceled
    (Class|VRCharacterBase|RightGrabReleased :!label _label)
    (Class|VRCharacterBase|UpdateRightHandPose 0.0 0.0))
  (:Completed
    (goto _label)))

(event EventBeginPlay)

(event Collision|EventActorBeginOverlap
  (params (OtherActor :type Actor%20Object%20Reference)))

(event EventTick
  (params (DeltaSeconds :type Float%20%28single-precision%29)))

(fn ConstructionScript)